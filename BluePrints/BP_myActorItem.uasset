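; BP_myActorItem is an item actor that holds wine info and hooks itself to BP_createActors spawner actors, with debug prints throughout.
; On BeginPlay it finds every BP_createActors and binds createEvent to its NewEventDispatcherCreator, behind a check on that actor's own first tag.
; PrintMyData prints the wine name and image fields from the MyInfoAA struct.
; Construction and PrintCreatedStatus only print creation messages.
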(event Collision|EventActorBeginOverlap
  (params (OtherActor :type Actor%20Object%20Reference)))

(event EventTick
  (params (DeltaSeconds :type Float%20%28single-precision%29)))

(event EventBeginPlay
  (Development|PrintString "BeginPlay Bind Start")
  (bind _outactors (Actor|GetAllActorsOfClass "/Game/BluePrints/BP_createActors.BP_createActors_C"))
  (for _array_element _outactors
    (Development|PrintString (Utilities|String|ToString(Name) (Utilities|Array|Get(acopy) (Variables|/Script/Engine.Actor|GetTags _array_element))))
    (if (Actor|ActorHasTag _array_element (Utilities|Array|Get(acopy) (Variables|/Script/Engine.Actor|GetTags _array_element)))
      (EventDispatchers|BindEventtoNewEventDispatcherCreator _array_element (EventDispatchers|CreateEvent :!event PrintMyData))
      (Development|PrintString "Bind Done"))))

(fn ConstructionScript
  (Development|PrintString "New Actor"))

(fn PrintMyData
  (Development|PrintString "Print My Data START")
  (bind _structout (Utilities|Struct|SetmembersinBP_ST_myEverwewStruct (Variables|Default|GetmyInfoAA)))
  (Development|PrintString (.wine_name (Utilities|Struct|BreakStructDataInfo (Utilities|Struct|BreakBP_ST_myEverwewStruct _structout))))
  (Development|PrintString (.wine_img (Utilities|Struct|BreakStructDataInfo (Utilities|Struct|BreakBP_ST_myEverwewStruct _structout))))
  (Development|PrintString "PrintMydata END"))

(fn PrintCreatedStatus
  (Development|PrintString "Im Actor Created"))