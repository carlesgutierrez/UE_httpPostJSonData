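; Debug-style spawner actor that creates BP_myActorItem actors from JSON data, apparently wine info, held by a MyHttpPostActor.
; On BeginPlay it enables player input and casts every MyHttpPostActor in the level to obtain that data source.
; X spawns an item, copies the last JSON request result into its struct and fires the NewEventDispatcherCreator dispatcher; P only fires the dispatcher.
; HTTP call, local JSON load and field-print nodes are left unconnected.
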(event Collision|EventActorBeginOverlap
  (params (OtherActor :type Actor%20Object%20Reference)))

(event EventTick
  (params (DeltaSeconds :type Float%20%28single-precision%29)))

(event EventBeginPlay
  (Input|EnableInput (Game|GetPlayerController 0))
  ;[1 1 1] Incomming Values Json
  (Development|PrintString "Incomming JSon Start")
  (bind _outactors (Actor|GetAllActorsOfClass "/Script/EasyBacchusAR.MyHttpPostActor"))
  (for _array_element _outactors
    (bind _asmy_http_post_actor (Utilities|Casting|CastToMyHttpPostActor _array_element)
      (:CastFailed
        (Development|PrintString "ERROR CASTING")))))

(event Input|KeyboardEvents|P
  (params (Key :type Key%20Structure))
  ;[1 1 1] Printing All Actors Data with Events
  (:Pressed
    (Default|CallNewEventDispatcherCreator)))

(event Input|KeyboardEvents|X
  (params (Key :type Key%20Structure))
  (:Pressed
    (bind _returnvalue (Game|SpawnActorfromClass "/Game/BluePrints/BP_myActorItem.BP_myActorItem_C" (Variables|Default|GetNewVar_0) "Undefined" 0 0))
    ;[1 1 1] Set values to MyStaticStruct VAR ( Load Data into new Actor ) with Events
    (Utilities|Struct|SetmembersinBP_ST_myEverwewStruct (Variables|/Game/BluePrints/BP_myActorItem.BP_myActorItem_C|GetmyInfoAA _returnvalue) (Variables|/Script/EasyBacchusAR.MyHttpPostActor|GetmyLastJsonRequestResult (stale EventBeginPlay _asmy_http_post_actor)))
    (Default|CallNewEventDispatcherCreator)))

(fn ConstructionScript)